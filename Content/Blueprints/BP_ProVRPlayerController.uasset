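; BP_ProVRPlayerController is a player controller that holds a debug hotkey for finding and joining an online session.
; Pressing 1 runs an asynchronous non-LAN session search, prints the result count and first session ID, then joins that first result without an empty-list check.
; Success and failure are reported only through Print String; BeginPlay, Tick and a few leftover nodes, including an Open Level call, are inactive.
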(event Custom|CustomEvent_0)

(event EventBeginPlay)

(event EventTick
  (params (DeltaSeconds :type Float%20%28single-precision%29)))

(event Input|KeyboardEvents|1
  (params (Key :type Key%20Structure :default "None"))
  (:Pressed
    (bind _results (|FindSessions self 100 false)
      (:then
        (Development|PrintString "Hello"))
      (:OnSuccess
        (Development|PrintString (Utilities|String|ToString(Integer) (Utilities|Array|Length _results)))
        (Development|PrintString (Class|AdvancedSessionsLibrary|GetSessionIDasString (Utilities|Array|Get(acopy) _results)) true true "(R=0.000000,G=0.660000,B=1.000000,A=1.000000)" 1e+02)
        (|JoinSession self (Utilities|Array|Get(acopy) _results)
          (:OnSuccess
            (Development|PrintString "Session joined!" true true "(R=0.000000,G=0.660000,B=1.000000,A=1.000000)" 1e+02))
          (:OnFailure
            (Development|PrintString "Join session failed!"))))
      (:OnFailure
        (Development|PrintString "Find session failed!")))))

(fn ConstructionScript)