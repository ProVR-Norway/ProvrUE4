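; BP_ProVRGameMode is a game mode base class that queues startup actions on the ProVR action manager.
; Three seconds after BeginPlay, it constructs and queues a hello-world action, a switch-view action with no target view, and a Google HTTP request action.
; The HTTP action's completion delegate prints the success flag and response content length, so the sequence appears to act as a demo of the action queue.
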(event Custom|OnActionComplete_Event
  (params (Success :type Boolean) (Content :type String))
  (Development|PrintString (Utilities|String|Append "Request to google: " "Success? " (Utilities|String|ToString(Boolean) Success) ", content length: " (Utilities|String|ToString(Integer) (Utilities|String|Len Content)))))

(event EventBeginPlay
  (bind _self self)
  (Utilities|FlowControl|Delay 3.0)
  (Utilities|FlowControl|Sequence
    (:then_0
      (bind _returnvalue (Game|ConstructObjectfromClass "/Script/ProVR.ProVRHelloWorldAction" _self))
      (Class|ProVRActionManager|QueueAction (Class|ProVRGameInstance|GetActionManager) _returnvalue))
    (:then_1
      (bind _returnvalue_2 (Game|ConstructObjectfromClass "/Script/ProVR.ProVRSwitchViewAction" _self))
      (Variables|/Script/ProVR.ProVRSwitchViewAction|SetDesiredNextView _returnvalue_2 "None")
      (Class|ProVRActionManager|QueueAction (Class|ProVRGameInstance|GetActionManager) _returnvalue_2))
    (:then_2
      (bind _returnvalue_3 (Game|ConstructObjectfromClass "/Script/ProVR.ProVRGoogleHttpRequestAction" _self))
      (EventDispatchers|AssignOnActionComplete _returnvalue_3 (delegate Custom|OnActionComplete_Event))
      (Class|ProVRActionManager|QueueAction (Class|ProVRGameInstance|GetActionManager) _returnvalue_3))))

(fn ConstructionScript)