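; Player controller for a participant in a ProVR-based app, which switches to the session view when play begins.
; BeginPlay runs a custom event that constructs a ProVRSwitchViewAction owned by the game instance, with SessionView as the desired next view.
; The action is queued on the action manager rather than changing the view directly.
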(event Custom|Create%20session%20view
  (bind _returnvalue (Game|ConstructObjectfromClass "/Script/ProVR.ProVRSwitchViewAction" (Game|GetGameInstance)))
  (Variables|/Script/ProVR.ProVRSwitchViewAction|SetDesiredNextView _returnvalue "SessionView")
  (Class|ProVRActionManager|QueueAction (Class|ProVRGameInstance|GetActionManager) _returnvalue))

(event EventBeginPlay
  (|CallParentFunction)
  (CallFunction|CreateSessionView))

(event EventTick
  (params (DeltaSeconds :type Float%20%28single-precision%29))
  (|CallParentFunction DeltaSeconds) ; This node is disabled and will not be called.\nDrag off pins to build functionality.
)

(fn ConstructionScript
  (|CallParentFunction))